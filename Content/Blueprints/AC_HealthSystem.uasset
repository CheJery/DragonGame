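; AC_HealthSystem is an actor component that tracks health and death for its owning actor.
; On begin play it binds to the owner's any-damage event and passes damage as a negative adjustment.
; AdjustHealth clamps current health between zero and the maximum and triggers Death at zero.
; Death only sets a dead flag and prints debug text, as damage handling also prints current health.
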(event `self.ReceiveBeginPlay`
  (add `Actor.OnTakeAnyDamage` (`self.GetOwner`) (delegate `OnDamageTaken`)))

(event `OnDamageTaken`
  (params (DamagedActor :type "Actor Object Reference") (Damage :type "Float (single-precision)") (DamageType :type "DamageType Object Reference") (InstigatedBy :type "Controller Object Reference") (DamageCauser :type "Actor Object Reference"))
  (`self.AdjustHealth` (* Damage -1.0))
  (`KismetSystemLibrary.PrintString` (`KismetStringLibrary.Conv_DoubleToString` (`self.currentHealth`))))

(event `AdjustHealth`
  (params (`Health Added` :type "Float (double-precision)"))
  (set `self.currentHealth` (`KismetMathLibrary.FClamp` (+ `Health Added` (`self.currentHealth`)) 0.0 (`self.maxHealth`)))
  (if (<= (`self.currentHealth`) 0.0)
    (`self.Death`)))

(event `Death`
  (set `self.isDead` true)
  (`KismetSystemLibrary.PrintString` "Dead"))