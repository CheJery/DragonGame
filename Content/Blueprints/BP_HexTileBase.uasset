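; BP_HexTileBase is a base hex tile actor that stores X/Y grid coordinates and references a health system component, ACHealthSystem.
; Every Tick it draws two black debug strings: the grid coordinates at the actor location and current/max health slightly above.
; It contains no other active logic, as BeginPlay, overlap and the construction script are empty.
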(event `self.ReceiveTick`
  (params (DeltaSeconds :type "Float (single-precision)"))
  (`KismetSystemLibrary.DrawDebugString` (`self.K2_GetActorLocation`) (`KismetStringLibrary.Concat_StrStr` (`KismetStringLibrary.Conv_IntToString` (`self.X-Grid`)) ", " (`KismetStringLibrary.Conv_IntToString` (`self.Y-Grid`))) null (struct :`A` 1.0))
  (`KismetSystemLibrary.DrawDebugString` (+ (`self.K2_GetActorLocation`) (0.0 0.0 20.0)) (`KismetStringLibrary.Concat_StrStr` (`KismetStringLibrary.Conv_DoubleToString` (`/Game/Blueprints/AC_HealthSystem.currentHealth` (`self.AC_HealthSystem`))) " / " (`KismetStringLibrary.Conv_DoubleToString` (`/Game/Blueprints/AC_HealthSystem.maxHealth` (`self.AC_HealthSystem`)))) null (struct :`A` 1.0)))

(fn `UserConstructionScript`)