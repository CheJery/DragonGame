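; Hex grid manager that spawns a grid of randomly chosen landscape, urban, water or base tiles at BeginPlay.
; Weighted random selection picks each tile class, and each tile receives its grid coordinates.
; Placement uses the mesh-derived radius, scale and gap offset, with a FlipFlop staggering alternate rows.
; After each spawn, it filters ActorArray to landscape tiles and prunes those far from a single found urban tile.
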(event `self.ReceiveBeginPlay`
  (bind (_returnvalue_x _returnvalue_y _returnvalue_z) (`KismetMathLibrary.BreakVector` (`SceneComponent.K2_GetComponentLocation` (`self.DefaultSceneRoot`))))
  ;[1 1 1] Taking Radius from Mesh
  (set `self.Radius` (* (.x (`.Max` (break `Box` (`StaticMesh.GetBoundingBox` (`self.Tile Mesh`))))) (`self.Scale`)))
  ;[1 1 1] Grid Height Loop
  (for _index (range (`self.GridHeight`))
    ;[1 1 1] Width Loop
    (for _index_2 (range (`self.GridWidth`))
      ;[1 1 1] Weighted Actor Randomizer
      (bind _sum_of_values (`self.SumValues`))
      (bind _indexthatwon (`self.DetermineIndex` (`KismetMathLibrary.RandomFloatInRange` 0.0 _sum_of_values)))
      (bind _asbp_hex_tile_base (castclass `/Game/Blueprints/BP_HexTileBase` (select `int` _indexthatwon :`0` (`self.Landscape Tile`) :`1` (`self.Urban Tile`) :`2` (`self.Water Tile`) :`3` (`self.Base Tile`))))
      ;[1 1 1] Spawn Actor
      (bind _returnvalue (`|SpawnActorFromClass` _asbp_hex_tile_base (`KismetMathLibrary.MakeTransform` (`KismetMathLibrary.MakeVector` (+ (+ (* _index_2 (`self.Radius`) 2.0) (* _index_2 (`self.Offset`)) (`self.RowOffset`)) _returnvalue_x) (+ _returnvalue_y (+ (* (/ (* (`self.Radius`) 2.0) (`KismetMathLibrary.Sqrt` 3.0)) 1.5 _index) (* _index (`self.Offset`)))) _returnvalue_z) (struct) (`KismetMathLibrary.Conv_DoubleToVector` (`self.Scale`))) "Undefined" "OverrideRootScale" null _index_2 _index null))
      (bind _output_get (set `self.ActorArray` (`self.ActorArray`)))
      (`KismetArrayLibrary.Array_Add` _output_get _returnvalue)
      (bind _filteredarray (`KismetArrayLibrary.FilterArray` (`self.ActorArray`) "/Game/Blueprints/BP_HexTileLandscape.BP_HexTileLandscape_C"))
      (bind _output_get_2 (set `self.ActorArray` _filteredarray))
      (for (_array_element _array_index) _output_get_2
        (bind _returnvalue_2 (`GameplayStatics.GetActorOfClass` "/Game/Blueprints/BP_HexTileUrban.BP_HexTileUrban_C"))
        (bind (_returnvalue_x_2 _returnvalue_y_2) (`KismetMathLibrary.BreakVector` (`self.K2_GetActorLocation` _array_element)))
        (bind (_returnvalue_x_3 _returnvalue_y_3) (`KismetMathLibrary.BreakVector` (`self.K2_GetActorLocation` _returnvalue_2)))
        (bind _output_get_3 (set `self.InCityProximityX` (> 1600.0 (`KismetMathLibrary.Abs` (- _returnvalue_x_2 _returnvalue_x_3)))))
        (bind _output_get_4 (set `self.InCityProximityY` (> 1600.0 (`KismetMathLibrary.Abs` (- _returnvalue_y_2 _returnvalue_y_3)))))
        (bind _output_get_5 (set `self.InCityProximity` (and _output_get_3 _output_get_4)))
        (if (not _output_get_5)
          (`KismetArrayLibrary.Array_Remove` (`self.ActorArray`) _array_index))))
    ;[1 1 1] Row Offset
    (`/Engine/EditorBlueprintResources/StandardMacros.FlipFlop`
      (:`A`
        (set `self.RowOffset` (* (`self.Radius`) -1.0)))
      (:`B`
        (set `self.RowOffset` 0.0)))))

(fn `DetermineIndex`
  (params (RandomValue :type "Float (double-precision)"))
  (returns (IndexThatWon :type Integer))
  (locals (LocalSum :type "Float (double-precision)"))
  (for (_array_element _array_index) (`self.WeightValues`)
    (bind _output_get (set `local.LocalSum` (+ _array_element (`local.LocalSum`))))
    (if (>= _output_get RandomValue)
      (break)))
  (return _array_index))

(fn `SumValues`
  (returns (`Sum of Values` :type "Float (double-precision)"))
  (locals (LocalSum :type "Float (double-precision)"))
  (for _array_element (`self.WeightValues`)
    (set `local.LocalSum` (+ _array_element (`local.LocalSum`))))
  (return (`local.LocalSum`)))

(fn `UserConstructionScript`)